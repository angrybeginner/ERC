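; Prototype vehicle body actor that generates a randomized six-wheel layout when play begins.
; CreateWheels spawns a wheel actor near each front, middle and back anchor, randomizing position within range widths and scale per axis.
; Spawn points add anchor relative locations to the body's world location, ignoring body rotation, and wheels are stored without attachment.
; Two physics handles then issue grab calls with no target component specified.
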(event EventBeginPlay
  (CallFunction|CreateWheels)
  (Class|PhysicsHandleComponent|GrabComponentatLocation (Variables|Default|GetPhysicsHandle) 0 "None" "0, 0, 0")
  (Class|PhysicsHandleComponent|GrabComponentatLocation (Variables|Default|GetPhysicsHandle1) 0 "None" "0, 0, 0"))

(fn ConstructionScript)

(fn CreateWheels
  (bind _wheelrange_y_width (Variables|Default|GetWheelRange_Y_Width))
  (bind _wheelrange_x_width (Variables|Default|GetWheelRange_X_Width))
  (bind _wheelrange_z_width (Variables|Default|GetWheelRange_Z_Width))
  (bind _wheelscale_min (Variables|Default|GetWheelScale_Min))
  (bind _wheelscale_max (Variables|Default|GetWheelScale_Max))
  (bind _returnvalue (/ _wheelrange_y_width 2.0))
  (bind _returnvalue_2 (/ _wheelrange_x_width 2.0))
  (bind _returnvalue_3 (/ _wheelrange_z_width 2.0))
  (bind _returnvalue_4 (Math|Random|RandomFloatinRange _wheelscale_min _wheelscale_max))
  (bind _output_get (Variables|Default|SetMyWheelPosition_Array (Utilities|Array|MakeArray (Variables|Default|GetFront%20Left%20Wheel) (Variables|Default|GetMiddle%20Right%20Wheel) (Variables|Default|GetMiddle%20Left%20Wheel) (Variables|Default|GetBack%20Left%20Wheel) (Variables|Default|GetBack%20Right%20Wheel) (Variables|Default|GetFront%20Right%20Wheel))))
  (for _array_element _output_get
    (bind _returnvalue_5 (Game|SpawnActorfromClass "/Game/GraphicSource/Wheel/temp_Wheel_BP.temp_Wheel_BP_C" (Math|Transform|MakeTransform (+ (Transformation|GetWorldLocation (Variables|Default|GetCarBody)) (Math|Vector|MakeVector (Math|Random|RandomFloatinRange (+ (.X (Math|Vector|BreakVector (Variables|/Script/Engine.SceneComponent|GetRelativeLocation _array_element))) (* -1 _returnvalue_2)) (+ (.X (Math|Vector|BreakVector (Variables|/Script/Engine.SceneComponent|GetRelativeLocation _array_element))) _returnvalue_2)) (Math|Random|RandomFloatinRange (+ (.Y (Math|Vector|BreakVector (Variables|/Script/Engine.SceneComponent|GetRelativeLocation _array_element))) (* -1 _returnvalue)) (+ (.Y (Math|Vector|BreakVector (Variables|/Script/Engine.SceneComponent|GetRelativeLocation _array_element))) _returnvalue)) (Math|Random|RandomFloatinRange (+ (.Z (Math|Vector|BreakVector (Variables|/Script/Engine.SceneComponent|GetRelativeLocation _array_element))) (* -1 _returnvalue_3)) (+ (.Z (Math|Vector|BreakVector (Variables|/Script/Engine.SceneComponent|GetRelativeLocation _array_element))) _returnvalue_3)))) "0,0.000000, 0" (Math|Vector|MakeVector _returnvalue_4 _returnvalue_4 _returnvalue_4)) "Undefined" 0 0))
    (Utilities|Array|Add (Variables|Default|GetMyWheels) _returnvalue_5)))