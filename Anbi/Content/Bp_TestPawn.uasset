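; Test pawn that suspends four physics-driven wheel actors from its own attachment points.
; On BeginPlay a reused macro spawns half-scale Temp_Wheel_BP actors at three arrows and Point1, stores them in MyWheels and grabs each Wheel with its own PhysicsHandle.
; A one-off impulse then pushes Cube at Arrow3's location.
; Every Tick moves the handle targets to those points and forces the wheel actors to zero rotation with physics teleport.
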(event EventBeginPlay
  (bind _returnvalue (Utilities|새매크로0 (Variables|Default|GetArrow) (Variables|Default|GetPhysicsHandle))
    (:NewParam2
      (bind _returnvalue_2 (Utilities|새매크로0 (Variables|Default|GetArrow2) (Variables|Default|GetPhysicsHandle1))
        (:NewParam2
          (bind _returnvalue_3 (Utilities|새매크로0 (Variables|Default|GetArrow1) (Variables|Default|GetPhysicsHandle2))
            (:NewParam2
              (bind _returnvalue_4 (Utilities|새매크로0 (Variables|Default|Getpoint%201) (Variables|Default|GetPhysicsHandle3))
                (:NewParam2
                  (Physics|AddImpulseatLocation (Variables|Default|GetCube) "-10000.000000, 0,0.000000" (Transformation|GetWorldLocation (Variables|Default|GetArrow3)) "None"))))))))))

(event EventTick
  (params (DeltaSeconds :type Float%20%28single-precision%29))
  (Class|PhysicsHandleComponent|SetTargetLocationandRotation (Variables|Default|GetPhysicsHandle) (Transformation|GetWorldLocation (Variables|Default|GetArrow)) "0, 0, 0")
  (Class|PhysicsHandleComponent|SetTargetLocationandRotation (Variables|Default|GetPhysicsHandle1) (Transformation|GetWorldLocation (Variables|Default|GetArrow2)) "0, 0, 0")
  (Class|PhysicsHandleComponent|SetTargetLocationandRotation (Variables|Default|GetPhysicsHandle2) (Transformation|GetWorldLocation (Variables|Default|GetArrow1)) "0, 0, 0")
  (Class|PhysicsHandleComponent|SetTargetLocationandRotation (Variables|Default|GetPhysicsHandle3) (Transformation|GetWorldLocation (Variables|Default|Getpoint%201)) "0, 0, 0")
  (Transformation|SetActorRotation (stale EventBeginPlay _returnvalue) "0, 0, 0" true)
  (Transformation|SetActorRotation (stale EventBeginPlay _returnvalue_2) "0,0.000000, 0" true)
  (Transformation|SetActorRotation (stale EventBeginPlay _returnvalue_3) "0, 0, 0" true)
  (Transformation|SetActorRotation (stale EventBeginPlay _returnvalue_4) "0, 0, 0" true))

(fn ConstructionScript)